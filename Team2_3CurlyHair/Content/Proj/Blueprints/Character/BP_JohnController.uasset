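; Player controller for John that handles walking and charged jumps, pushes animation states to the character, and routes pause and height progress to the HUD.
; Holding jump blocks walking and adds a fixed step per Triggered event, so charge depends on tick rate.
; Release or maximum hold launches the grounded character, scaling vertical velocity by charge and taking horizontal direction from the last MovementBuffer entry.
; A looping timer reports the character's Z to the HUD.
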(event Custom|PlayerJump
  (CallFunction|SetPlayerAnimState "NewEnumerator4")
  (CallFunction|SwitchInputBuffer)
  (Character|LaunchCharacter (Game|GetPlayerCharacter 0) (Math|Vector|MakeVector (Variables|Default|GethorizontalLaunch) 0.0 (* (Variables|Default|GetspaceBarSecondsHeld) 2.5e+02)) false false)
  (Audio|PlaySound2D "/Game/Proj/SFX/MetaSounds/MS_Launch.MS_Launch" 1.0 1.0 0.0 0 0)
  (Development|PrintString "Launch")
  (CallFunction|ZeroValuesAfterLaunch))

(event Custom|StartProgressUpdateTimer
  (Utilities|Time|SetTimerbyEvent (delegate Custom|ProgressUpdateTimer) 0.3 true))

(event Custom|ProgressUpdateTimer
  (Class|BPIHUD|UpdatePlayerProgress(Message) (HUD|GetHUD) (.z (Transformation|GetActorLocation (Game|GetPlayerCharacter 0)))))

(event Input|EnhancedActionEvents|EnhancedInputActionIA_Pause
  (params (ActionValue :type Boolean) (ElapsedSeconds :type Float%20%28double-precision%29) (TriggeredSeconds :type Float%20%28double-precision%29) (InputAction :type Input%20Action%20Object%20Reference :default "/Game/Proj/Blueprints/Character/Input/InputActions/IA_Pause.IA_Pause"))
  (:Started
    (Class|BPIHUD|SetNewWidget(Message) (HUD|GetHUD) "NewEnumerator0")))

(event Input|EnhancedActionEvents|EnhancedInputActionIA_Left
  (params (ActionValue :type Float%20%28double-precision%29) (ElapsedSeconds :type Float%20%28double-precision%29) (TriggeredSeconds :type Float%20%28double-precision%29) (InputAction :type Input%20Action%20Object%20Reference :default "/Game/Proj/Blueprints/Character/Input/InputActions/IA_Left.IA_Left"))
  (:Triggered
    (CallFunction|PlayerMoveLeft ActionValue))
  (:Started
    (CallFunction|LeftInputStarted)
    (if (not (Variables|Default|GetjumpButtonTriggered))
      (CallFunction|SetPlayerAnimState "NewEnumerator0")))
  (:Completed
    (CallFunction|LeftInputCompleted)
    (CallFunction|InputCompleted)))

(event Input|EnhancedActionEvents|EnhancedInputActionIA_Right
  (params (ActionValue :type Float%20%28double-precision%29) (ElapsedSeconds :type Float%20%28double-precision%29) (TriggeredSeconds :type Float%20%28double-precision%29) (InputAction :type Input%20Action%20Object%20Reference :default "/Game/Proj/Blueprints/Character/Input/InputActions/IA_Right.IA_Right"))
  (:Triggered
    (CallFunction|PlayerMoveRight ActionValue))
  (:Started
    (CallFunction|RightInputStarted)
    (if (not (Variables|Default|GetjumpButtonTriggered))
      (CallFunction|SetPlayerAnimState "NewEnumerator0")))
  (:Completed
    (CallFunction|RightInputCompleted)
    (CallFunction|InputCompleted)))

(event Input|EnhancedActionEvents|EnhancedInputActionIA_Jump
  (params (ActionValue :type Boolean) (ElapsedSeconds :type Float%20%28double-precision%29) (TriggeredSeconds :type Float%20%28double-precision%29) (InputAction :type Input%20Action%20Object%20Reference :default "/Game/Proj/Blueprints/Character/Input/InputActions/IA_Jump.IA_Jump"))
  (:Triggered
    (if (Utilities|PlayerIsNotFalling)
      (Variables|Default|SetjumpButtonTriggered true)
      (bind _output_get (CallFunction|CalculateVariableJumpTimer))
      (if (>= _output_get (Variables|Default|GetMaxTimerHold))
        (CallFunction|PlayerJump))))
  (:Started
    (Audio|PlaySound2D "/Game/Proj/SFX/MetaSounds/MS_PreLaunch.MS_PreLaunch" 1.0 1.0 0.0 0 0)
    (if (Utilities|PlayerIsNotFalling)
      (CallFunction|DetermineLRCPreLaunch)))
  (:Canceled
    (Variables|Default|SetjumpButtonTriggered false))
  (:Completed
    (CallFunction|JumpButtonCompleted)))

(event EventBeginPlay
  (bind _returnvalue (PlayerController|LocalPlayerSubsystems|GetEnhancedInputLocalPlayerSubsystem))
  (Utilities|IsValid _returnvalue
    (:Is%20Valid
      (Input|AddMappingContext _returnvalue "/Game/Proj/Blueprints/Character/Input/IM_JohnMappingContext.IM_JohnMappingContext" 0 "(bIgnoreAllPressedKeysUntilRelease=True,bForceImmediately=False,bNotifyUserSettings=False)")
      (CallFunction|StartProgressUpdateTimer)
      (Class|BPIPlayerInterface|SetPlayerGravityLevel(Message) (Game|GetPlayerCharacter 0) 1.8))))

(fn ConstructionScript)

(fn SwitchInputBuffer
  (bind _movementbuffer (Variables|Default|GetmovementBuffer))
  (bind _returnvalue (Utilities|Array|Length _movementbuffer))
  (if (> _returnvalue 0)
    _
    (else
      (Utilities|Array|Add (Variables|Default|GetmovementBuffer) "NewEnumerator2")))
  (switch Utilities|FlowControl|Switch|SwitchonE_MovementBuffer (Utilities|Array|Get(acopy) (Variables|Default|GetmovementBuffer) (- _returnvalue 1))
    (:NewEnumerator0
      (Variables|Default|SethorizontalLaunch (* (Variables|Default|GethorizontalLaunchSpeed) -1.0)))
    (:NewEnumerator1
      (Variables|Default|SethorizontalLaunch (Variables|Default|GethorizontalLaunchSpeed)))
    (:NewEnumerator2
      (Variables|Default|SethorizontalLaunch 0.0))))

(fn ZeroValuesAfterLaunch
  (Variables|Default|SetspaceBarSecondsHeld 0.0)
  (Variables|Default|Settimer 0.0)
  (Utilities|Array|Clear (Variables|Default|GetmovementBuffer))
  (Variables|Default|SethorizontalLaunch 0.0))

(fn RightInputCompleted
  (Variables|Default|SetrightButtonTriggered false)
  (if (not (Variables|Default|GetleftButtonTriggered))
    (Utilities|Array|Add (Variables|Default|GetmovementBuffer) "NewEnumerator1")
    (Development|PrintString "center")))

(fn LeftInputCompleted
  (Variables|Default|SetleftButtonTriggered false)
  (if (not (Variables|Default|GetrightButtonTriggered))
    (Utilities|Array|Add (Variables|Default|GetmovementBuffer) "NewEnumerator2")
    (Development|PrintString "center")))

(fn LeftInputStarted
  (Utilities|Array|Add (Variables|Default|GetmovementBuffer) "NewEnumerator0")
  (Development|PrintString "left"))

(fn RightInputStarted
  (Utilities|Array|Add (Variables|Default|GetmovementBuffer) "NewEnumerator1")
  (Development|PrintString "right"))

(fn PlayerMoveRight
  (params (ScaleValue :type Float%20%28single-precision%29))
  (bind (_player _worlddirection) (Utilities|PlayerMoveRightInfo))
  (Variables|Default|SetrightButtonTriggered true)
  (if (not (Variables|Default|GetjumpButtonTriggered))
    (Pawn|Input|AddMovementInput _player _worlddirection ScaleValue false)))

(fn PlayerMoveLeft
  (params (ScaleValue :type Float%20%28single-precision%29))
  (bind (_player _worlddirection) (Utilities|PlayerMoveLeftInfo))
  (Variables|Default|SetleftButtonTriggered true)
  (if (not (Variables|Default|GetjumpButtonTriggered))
    (Pawn|Input|AddMovementInput _player _worlddirection ScaleValue false)))

(fn CalculateVariableJumpTimer
  (if (Utilities|PlayerIsNotFalling)
    (bind _output_get (Variables|Default|Settimer (+ (Variables|Default|Gettimer) 0.1)))
    (bind _output_get_2 (Variables|Default|SetspaceBarSecondsHeld _output_get)))
  (return _output_get_2))

(fn JumpButtonCompleted
  (Variables|Default|SetjumpButtonTriggered false)
  (if (Utilities|PlayerIsNotFalling)
    (CallFunction|PlayerJump)))

(fn SetPlayerAnimState
  (params (NewState :type E_PlayerAnimState%20Enum :default "NewEnumerator0"))
  (Class|BPIPlayerInterface|SetPlayerAnimState(Message) (Game|GetPlayerCharacter 0) NewState))

(fn InputStarted)

(fn InputCompleted
  (CallFunction|SetPlayerAnimState "NewEnumerator0"))

(fn DetermineLRCPreLaunch
  (bind _movementbuffer (Variables|Default|GetmovementBuffer))
  (bind _returnvalue (Utilities|Array|Length _movementbuffer))
  (if (> _returnvalue 0)
    _
    (else
      (Utilities|Array|Add (Variables|Default|GetmovementBuffer) "NewEnumerator2")))
  (switch Utilities|FlowControl|Switch|SwitchonE_MovementBuffer (Utilities|Array|Get(acopy) (Variables|Default|GetmovementBuffer) (- _returnvalue 1))
    (:NewEnumerator0
      (CallFunction|SetPlayerAnimState "NewEnumerator8"))
    (:NewEnumerator1
      (CallFunction|SetPlayerAnimState "NewEnumerator7"))
    (:NewEnumerator2
      (CallFunction|SetPlayerAnimState "NewEnumerator3"))))